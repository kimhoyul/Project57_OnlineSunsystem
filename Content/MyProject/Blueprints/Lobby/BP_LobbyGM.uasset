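; BP_LobbyGM is the lobby game mode that moves connected players from the lobby into the InGame map.
; On BeginPlay it calls EndSession with the first player controller.
; ShowLoading stops the timer, tells each player's BP_LobbyPC to create a loading screen, then calls StartInGame.
; StartInGame starts the advanced session and, on success, runs a ServerTravel console command to InGame.
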(event `self.ReceiveBeginPlay`
  (`EndSessionCallbackProxy.EndSession` (`GameplayStatics.GetPlayerController` 0)))

(event `StartInGame`
  (`StartSessionCallbackProxyAdvanced.StartAdvancedSession`
    (:`OnSuccess`
      (`KismetSystemLibrary.ExecuteConsoleCommand` (`KismetStringLibrary.Concat_StrStr` "ServerTravel " "InGame") null))))

(fn `ShowLoading`
  (`self.StopTimer`)
  (for _array_element (`GameStateBase.PlayerArray` (`GameplayStatics.GetGameState`))
    (bind _asbp_lobby_pc (cast `/Game/MyProject/Blueprints/Lobby/BP_LobbyPC` (`PlayerState.GetPlayerController` _array_element)))
    (`/Game/MyProject/Blueprints/Lobby/BP_LobbyPC.S2C_CreateLoadingScreen` _asbp_lobby_pc))
  (`self.StartInGame`))

(fn `UserConstructionScript`)